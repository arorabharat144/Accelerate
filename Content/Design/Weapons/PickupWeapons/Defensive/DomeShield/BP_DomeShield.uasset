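; BP_DomeShield is a defensive pickup weapon that deploys a timed dome shield to protect the player's car.
; Firing activates a collision sphere and dome mesh, grown by timeline, then resets after a duration and re-arms after a cooldown.
; Overlapping laser projectiles are destroyed, while ShieldEffects animates an impact ripple through a dynamic material.
; The owning player's IsShieldActive flag clears only after the cooldown, later than the dome itself.
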(event `Init`
  (bind _spherecollision (`self.SphereCollision`))
  (bind _spheretexture (`self.SphereTexture`))
  (`ActorComponent.Deactivate` _spherecollision)
  (`SphereComponent.SetSphereRadius` _spherecollision 0.0 true)
  (`SceneComponent.SetRelativeScale3D` _spheretexture (0.1 0.1 0.1))
  (`ActorComponent.Deactivate` _spheretexture))

(event `self.ReceiveBeginPlay`
  (`self.Init`)
  (set `self.isReady` true))

(event `self.DomeShieldFire`
  (bind _spherecollision (`self.SphereCollision`))
  (bind _spheretexture (`self.SphereTexture`))
  ;[1 1 1] Deploy Shield Event
  (if (`self.isReady`)
    (set `self.isDomeShieldActive` true)
    (`|ExecutionSequence`
      (:`then_0`
        (`GameplayStatics.PlaySoundAtLocation` (`self.ShieldSound`) (`SceneComponent.K2_GetComponentLocation` (`self.SphereCollision`)) (struct) 1.0 1.0 0.0 null null null)
        (`ActorComponent.Activate` _spherecollision true)
        (`ActorComponent.Activate` _spheretexture true)
        (set `self.isReady` false)
        (set `AcceleratePlayer.isShieldActive` true (`self.GetOwningPlayer`)))
      (:`then_1`
        (bind (_direction _lerpamount) (`Timeline|Timeline_0` :!via `PlayFromStart`)
          (:`Update`
            (`SphereComponent.SetSphereRadius` _spherecollision (`KismetMathLibrary.Lerp` 0.0 (`self.sphereRadius`) _lerpamount) true)
            (`SceneComponent.SetRelativeScale3D` _spheretexture (`KismetMathLibrary.VLerp` (0.1 0.1 0.1) (`self.SphereTextureScale`) _lerpamount)))
          (:`Finished`
            (`KismetSystemLibrary.Delay` (`self.shieldDuration`))
            (set `self.isDomeShieldActive` false)
            (`self.Init`)
            (`KismetSystemLibrary.Delay` (`self.cooldown`))
            (set `self.isReady` true)
            (set `AcceleratePlayer.isShieldActive` false (`self.GetOwningPlayer`))))))))

(event `self.SphereCollision.OnComponentBeginOverlap`
  (params (OverlappedComponent :type "PrimitiveComponent Object Reference") (OtherActor :type "Actor Object Reference") (OtherComp :type "PrimitiveComponent Object Reference") (OtherBodyIndex :type Integer) (bFromSweep :type Boolean) (SweepResult :type "HitResult Structure (by ref)"))
  (`|ExecutionSequence`
    (:`then_1`
      ;[1 1 1] check for colision to stop damage to the car
      (bind _asbp_laser_projectile_69 (cast `/Game/Design/Weapons/BaseWeapons/Offensive/LaserBlaster/BP_LaserProJectile69` OtherActor))
      (`self.K2_DestroyActor` _asbp_laser_projectile_69))))

(event `ShieldEffects`
  (params (ImpactVector :type "Vector Structure"))
  ;[1 1 1] this part is just for the hit special effect
  (bind _returnvalue (`PrimitiveComponent.CreateDynamicMaterialInstance` (`self.SphereTexture`) 0 null "None"))
  (`MaterialInstanceDynamic.SetVectorParameterValue` _returnvalue "pos" (`KismetMathLibrary.Conv_VectorToLinearColor` ImpactVector))
  (bind (_direction _newtrack_0) (`Timeline|Timeline_1` :!via `PlayFromStart`)
    (:`Update`
      (`MaterialInstanceDynamic.SetScalarParameterValue` _returnvalue "radius" (* _newtrack_0 200.0)))))

(fn `UserConstructionScript`)