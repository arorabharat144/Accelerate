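; Homing missile projectile fired from a car-mounted weapon, taking its damage from that weapon.
; On spawn it adds the car's forward speed, then homes on the nearest AcceleratePlayer ahead of the car.
; A short forward trace each tick sets the projectile's plane constraint normal from blocking surfaces.
; Hits explode with a radial impulse and damage the target; overlaps damage players or trigger dome shield effects, destroying the missile.
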(event `self.ReceiveBeginPlay`
  (bind _projectile (`self.Projectile`))
  ;[1 1 1] Initializing Weapon and Car Owner
  (bind _asbp_homing_weapon_cpp (cast `/Game/Design/Weapons/PickupWeapons/Offensive/HomingMissile/BP_HomingWeaponCPP` (`self.GetOwner`)))
  (bind _output_get (set `self.FiringWeapon` _asbp_homing_weapon_cpp))
  (bind _aspawn (cast `Pawn` (`self.GetAttachParentActor` (`self.FiringWeapon`))))
  (set `self.WeaponDamage` (`HomingWeapon.damage` _output_get))
  (bind _output_get_2 (set `self.CarOwner` _aspawn))
  (`PrimitiveComponent.IgnoreActorWhenMoving` (`self.CollisionComponent`) (`self.CarOwner`) true)
  (bind _returnvalue (`self.GetVelocity` _output_get_2))
  (bind _returnvalue_2 (`self.GetActorForwardVector` _output_get_2))
  (if (> (`KismetMathLibrary.Dot_VectorVector` (`KismetMathLibrary.Normal` _returnvalue) _returnvalue_2) 0.0)
    (bind _output_get_3 (set `ProjectileMovementComponent.InitialSpeed` (+ (* (`KismetMathLibrary.Dot_VectorVector` _returnvalue _returnvalue_2) 1.0) (`ProjectileMovementComponent.InitialSpeed` _projectile)) _projectile))
    (set `ProjectileMovementComponent.MaxSpeed` (+ _output_get_3 2000.0) _projectile)
    (bind _returnvalue_3 (* (0.0 0.0 1.0) _output_get_3))
    (if (< (`KismetMathLibrary.VSize` _returnvalue_3) 5000.0)
      (bind _target (`self.FindTarget` :!label _label))
      (if (`KismetSystemLibrary.IsValid` _target)
        (bind _output_get_4 (set `self.Target` _target))
        (`self.HomingMissile` _output_get_4)
        (`self.SetLifeSpan` 10.0))
      (else
        (`ProjectileMovementComponent.SetVelocityInLocalSpace` _projectile _returnvalue_3)
        (bind _target_2 (`self.FindTarget`))
        (if (`KismetSystemLibrary.IsValid` _target_2)
          (bind _output_get_5 (set `self.Target` _target_2))
          (`self.HomingMissile` _output_get_5)
          (`self.SetLifeSpan` 10.0))))
    (else
      (goto _label))))

(event `self.CollisionComponent.OnComponentHit`
  (params (HitComponent :type "PrimitiveComponent Object Reference") (OtherActor :type "Actor Object Reference") (OtherComp :type "PrimitiveComponent Object Reference") (NormalImpulse :type "Vector Structure") (Hit :type "HitResult Structure (by ref)"))
  (bind _explosionforce (`self.ExplosionForce`))
  (bind _target (`self.Target`))
  ;[1 1 1] Explode on contact
  (if (and (!= OtherActor (`self.FiringWeapon`)) (!= OtherActor (`self.CarOwner`)))
    (`PrimitiveComponent.SetCollisionEnabled` (`self.CollisionComponent`) "QueryAndPhysics")
    (`/Engine/EditorBlueprintResources/StandardMacros.DoOnce` false
      (:`Completed`
        (`RadialForceComponent.FireImpulse` _explosionforce)
        (`GameplayStatics.SpawnEmitterAtLocation` "/Game/StarterContent/Particles/P_Explosion.P_Explosion" (`SceneComponent.K2_GetComponentLocation` _explosionforce))
        (if (and (`KismetSystemLibrary.IsValid` _target) (== OtherActor _target))
          (`AcceleratePlayer.ReceiveDamage` _target (`self.WeaponDamage`))
          (`self.K2_DestroyActor`)
          (else
            (`self.K2_DestroyActor`)))))))

(event `HomingMissile`
  (params (TargetToHit :type "AcceleratePlayer Object Reference"))
  (bind _projectile (`self.Projectile`))
  ;[1 1 1] Set Homing Missile
  (if (`KismetSystemLibrary.IsValid` TargetToHit)
    (set `ProjectileMovementComponent.HomingTargetComponent` (`Car.Mesh` TargetToHit) _projectile)
    (set `ProjectileMovementComponent.bIsHomingProjectile` true _projectile)
    (set `ProjectileMovementComponent.HomingAccelerationMagnitude` 50000.0 _projectile)))

(event `self.ReceiveTick`
  (params (DeltaSeconds :type "Float (single-precision)"))
  (bind _returnvalue (`self.K2_GetActorLocation`))
  (bind _outhit (`KismetSystemLibrary.LineTraceSingle` _returnvalue (+ _returnvalue (* (`SceneComponent.GetForwardVector` (`self.Sphere`)) 50.0)) "TraceTypeQuery1"))
  (bind (_bblockinghit _binitialoverlap _time _distance _location _impactpoint _normal _impactnormal) (`GameplayStatics.BreakHitResult` _outhit))
  (if _bblockinghit
    (`MovementComponent.SetPlaneConstraintNormal` (`self.Projectile`) _impactnormal)
    (else
      (`MovementComponent.SetPlaneConstraintNormal` (`self.Projectile`) (0.0 0.0 0.0)))))

(event `self.CollisionComponent.OnComponentBeginOverlap`
  (params (OverlappedComponent :type "PrimitiveComponent Object Reference") (OtherActor :type "Actor Object Reference") (OtherComp :type "PrimitiveComponent Object Reference") (OtherBodyIndex :type Integer) (bFromSweep :type Boolean) (SweepResult :type "HitResult Structure (by ref)"))
  (`|ExecutionSequence`
    (:`then_0`
      (if (== OtherActor (`self.CarOwner`))
        (`PrimitiveComponent.SetCollisionEnabled` (`self.CollisionComponent`) "QueryOnly")))
    (:`then_1`
      (bind _asbp_dome_shield (cast `/Game/Design/Weapons/PickupWeapons/Defensive/DomeShield/BP_DomeShield` OtherActor))
      (`/Game/Design/Weapons/PickupWeapons/Defensive/DomeShield/BP_DomeShield.ShieldEffects` _asbp_dome_shield SweepResult_ImpactPoint)
      (`self.K2_DestroyActor`))
    (:`then_2`
      (bind _asaccelerate_player (cast `AcceleratePlayer` OtherActor))
      (`AcceleratePlayer.ReceiveDamage` _asaccelerate_player (`self.WeaponDamage`))
      (`self.K2_DestroyActor`))))

(fn `FindTarget`
  (returns (Target :type "AcceleratePlayer Object Reference"))
  (locals (PossibleTargets :type "Array of /Game/Design/Car/BP_Car Object Reference") (minDistance :type "Float (double-precision)" :default 0.0) (targetCar :type "/Game/Design/Car/BP_Car Object Reference"))
  (bind _carowner (`self.CarOwner`))
  ;[1 1 1] Finding the closest target
  (if (not (`KismetSystemLibrary.IsValid` (`self.Target`)))
    (bind _outactors (`GameplayStatics.GetAllActorsOfClass` "/Script/Accelerate.AcceleratePlayer"))
    (bind _asaccelerate_player (cast `AcceleratePlayer` (`self.CarOwner`)))
    (`KismetArrayLibrary.Array_RemoveItem` _outactors _asaccelerate_player)
    (if (> (`KismetArrayLibrary.Array_Length` _outactors) 0)
      (set `local.minDistance` (`KismetMathLibrary.VSize` (- (`self.K2_GetActorLocation` (`|GetArrayItem` _outactors)) (`self.K2_GetActorLocation` _carowner))))
      (for _array_element _outactors
        (bind _returnvalue (- (`self.K2_GetActorLocation` _array_element) (`self.K2_GetActorLocation` _carowner)))
        (if (>= (`KismetMathLibrary.Dot_VectorVector` (`KismetMathLibrary.Normal` _returnvalue) (`SceneComponent.GetForwardVector` (`Actor.RootComponent` _carowner))) 0.0)
          (bind _returnvalue_2 (`KismetMathLibrary.VSize` _returnvalue))
          (if (<= _returnvalue_2 (`local.minDistance`))
            (set `local.minDistance` _returnvalue_2)
            (bind _output_get (set `self.Target` _array_element)))))
      (return _output_get))))

(fn `UserConstructionScript`)