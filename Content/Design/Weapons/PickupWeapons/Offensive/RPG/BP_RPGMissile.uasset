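; Projectile missile fired by BP_RPGWeapon from a vehicle, taking damage from the weapon and inheriting the car's forward speed.
; A HomingMissile event steers it toward a given actor's mesh, while a per-tick forward trace sets the movement's plane constraint normal from nearby surfaces.
; Hits on anything but the weapon or owning car fire a radial impulse and explosion effect, damage only the stored Target, then destroy the missile.
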(event `self.ReceiveBeginPlay`
  (bind _projectilemovement (`self.ProjectileMovement`))
  ;[1 1 1] Initializing Weapon and Car Owner
  (bind _asbp_rpgweapon (cast `/Game/Design/Weapons/PickupWeapons/Offensive/RPG/BP_RPGWeapon` (`self.GetOwner`)))
  (bind _output_get (set `self.FiringWeapon` _asbp_rpgweapon))
  (bind _aspawn (cast `Pawn` (`self.GetAttachParentActor` (`self.FiringWeapon`))))
  (set `self.WeaponDamage` (`RPGWeapon.damage` _output_get))
  (bind _output_get_2 (set `self.CarOwner` _aspawn))
  (`PrimitiveComponent.IgnoreActorWhenMoving` (`self.CollisionComponent`) (`self.CarOwner`) true)
  (bind _returnvalue (`self.GetVelocity` _output_get_2))
  (bind _returnvalue_2 (`self.GetActorForwardVector` _output_get_2))
  (if (> (`KismetMathLibrary.Dot_VectorVector` (`KismetMathLibrary.Normal` _returnvalue) _returnvalue_2) 0.0)
    (bind _output_get_3 (set `ProjectileMovementComponent.InitialSpeed` (+ (* (`KismetMathLibrary.Dot_VectorVector` _returnvalue _returnvalue_2) 1.0) (`ProjectileMovementComponent.InitialSpeed` _projectilemovement)) _projectilemovement))
    (set `ProjectileMovementComponent.MaxSpeed` (+ _output_get_3 2000.0) _projectilemovement)
    (bind _returnvalue_3 (* (0.0 0.0 1.0) _output_get_3))
    (if (< (`KismetMathLibrary.VSize` _returnvalue_3) 5000.0)
      (`ProjectileMovementComponent.SetVelocityInLocalSpace` (`self.ProjectileMovement`) _returnvalue_3)
      (`self.SetLifeSpan` 10.0))))

(event `self.CollisionComponent.OnComponentHit`
  (params (HitComponent :type "PrimitiveComponent Object Reference") (OtherActor :type "Actor Object Reference") (OtherComp :type "PrimitiveComponent Object Reference") (NormalImpulse :type "Vector Structure") (Hit :type "HitResult Structure (by ref)"))
  (bind _explosionforce (`self.ExplosionForce`))
  (bind _target (`self.Target`))
  ;[1 1 1] Explode on contact
  (if (and (!= OtherActor (`self.FiringWeapon`)) (!= OtherActor (`self.CarOwner`)))
    (`PrimitiveComponent.SetCollisionEnabled` (`self.CollisionComponent`) "QueryAndPhysics")
    (`/Engine/EditorBlueprintResources/StandardMacros.DoOnce` false
      (:`Completed`
        (`RadialForceComponent.FireImpulse` _explosionforce)
        (`GameplayStatics.SpawnEmitterAtLocation` "/Game/StarterContent/Particles/P_Explosion.P_Explosion" (`SceneComponent.K2_GetComponentLocation` _explosionforce))
        (if (and (`KismetSystemLibrary.IsValid` null) (== OtherActor _target))
          (`AcceleratePlayer.ReceiveDamage` _target (`self.WeaponDamage`))
          (`self.K2_DestroyActor`)
          (else
            (`self.K2_DestroyActor`)))))))

(event `HomingMissile`
  (params (TargetToHit :type "AcceleratePlayer Object Reference"))
  (bind _projectilemovement (`self.ProjectileMovement`))
  ;[1 1 1] Set Homing Missile
  (if (`KismetSystemLibrary.IsValid` TargetToHit)
    (set `ProjectileMovementComponent.HomingTargetComponent` (`Car.Mesh` TargetToHit) _projectilemovement)
    (set `ProjectileMovementComponent.bIsHomingProjectile` true _projectilemovement)
    (set `ProjectileMovementComponent.HomingAccelerationMagnitude` 50000.0 _projectilemovement)))

(event `self.ReceiveTick`
  (params (DeltaSeconds :type "Float (single-precision)"))
  (bind _returnvalue (`self.K2_GetActorLocation`))
  (bind _projectilemovement (`self.ProjectileMovement`))
  (bind _outhit (`KismetSystemLibrary.LineTraceSingle` _returnvalue (+ _returnvalue (* (`SceneComponent.GetForwardVector` (`self.CollisionComponent`)) 50.0)) "TraceTypeQuery1"))
  (bind (_bblockinghit _binitialoverlap _time _distance _location _impactpoint _normal _impactnormal) (`GameplayStatics.BreakHitResult` _outhit))
  (if _bblockinghit
    (`MovementComponent.SetPlaneConstraintNormal` _projectilemovement _impactnormal)
    (else
      (`MovementComponent.SetPlaneConstraintNormal` _projectilemovement (0.0 0.0 0.0)))))

(event `self.CollisionComponent.OnComponentBeginOverlap`
  (params (OverlappedComponent :type "PrimitiveComponent Object Reference") (OtherActor :type "Actor Object Reference") (OtherComp :type "PrimitiveComponent Object Reference") (OtherBodyIndex :type Integer) (bFromSweep :type Boolean) (SweepResult :type "HitResult Structure (by ref)"))
  (if (== OtherActor (`self.CarOwner`))
    (`PrimitiveComponent.SetCollisionEnabled` (`self.CollisionComponent`) "QueryOnly")))

(fn `UserConstructionScript`)