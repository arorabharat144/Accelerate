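; BP_ShockwaveGun is a defensive weapon that emits an expanding shockwave to push other players away.
; Firing, when ready, activates the collision sphere and SphereText, then a timeline grows both with MRadius.
; Players overlapping the sphere, except the owner, get MPushForceVetor applied to their mesh at the impact point.
; When the timeline finishes, both components reset and the gun becomes ready after MCooldown.
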(event `Init`
  (bind _spherecollision (`self.SphereCollision`))
  (bind _spheretext (`self.SphereText`))
  (`ActorComponent.Deactivate` _spherecollision)
  (`SphereComponent.SetSphereRadius` _spherecollision 0.0 true)
  (`SceneComponent.SetRelativeScale3D` _spheretext (0.1 0.1 0.1))
  (`ActorComponent.Deactivate` _spheretext))

(event `self.ReceiveBeginPlay`
  (`self.Init`)
  (set `self.mIsReady` true))

(event `self.ShockwaveGunFire`
  (bind _spherecollision (`self.SphereCollision`))
  (bind _spheretext (`self.SphereText`))
  (bind _mradius (`self.mRadius`))
  (if (`self.mIsReady`)
    (`|ExecutionSequence`
      (:`then_0`
        (set `self.mIsReady` false)
        (`ActorComponent.Activate` _spherecollision true)
        (`ActorComponent.Activate` _spheretext true))
      (:`then_1`
        (bind (_direction _lerpamount) (`Timeline|Timeline_0` :`NewTime` 3.0 :!via `PlayFromStart`)
          (:`Update`
            (`SphereComponent.SetSphereRadius` _spherecollision (+ (`self.baseCollisionSize`) (`KismetMathLibrary.Lerp` 0.0 (+ _mradius 20.0) _lerpamount)) true)
            (`SceneComponent.SetRelativeScale3D` _spheretext (`KismetMathLibrary.VLerp` (0.1 0.1 0.1) (`KismetMathLibrary.Conv_DoubleToVector` _mradius) _lerpamount)))
          (:`Finished`
            (`self.Init`)
            (`KismetSystemLibrary.Delay` (`self.mCooldown`))
            (set `self.mIsReady` true)))))))

(event `self.SphereCollision.OnComponentBeginOverlap`
  (params (OverlappedComponent :type "PrimitiveComponent Object Reference") (OtherActor :type "Actor Object Reference") (OtherComp :type "PrimitiveComponent Object Reference") (OtherBodyIndex :type Integer) (bFromSweep :type Boolean) (SweepResult :type "HitResult Structure (by ref)"))
  (bind _asaccelerate_player (cast `AcceleratePlayer` OtherActor))
  (if (!= _asaccelerate_player (`self.GetOwningPlayer`))
    (`PrimitiveComponent.AddForceAtLocation` (`Car.Mesh` _asaccelerate_player) (`self.mPushForceVetor`) SweepResult_ImpactPoint "None")))

(fn `UserConstructionScript`)