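; BP_BackShield is a defensive weapon that deploys a box shield to intercept homing missiles.
; BackShieldFire, gated by CanShoot, activates and enlarges the collision box and cube mesh to their set sizes.
; Overlapping homing missiles are destroyed and their weapon damage is passed to ReceiveDamage.
; Tick calls KillShield while health is depleted, shrinking the shield and re-enabling firing after MaxCooldown, with no health reset in this graph.
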(event `self.ReceiveBeginPlay`
  (`self.Init`)
  (`self.SetCanShoot` true))

(event `self.ReceiveTick`
  (params (DeltaSeconds :type "Float (single-precision)"))
  (if (<= (`self.mHealth`) 0.0)
    (`self.KillShield`)))

(event `Init`
  (bind _boxcollision (`self.BoxCollision`))
  (bind _reset_size (`self.reset size`))
  (bind _cubetexture (`self.CubeTexture`))
  ;[1 1 1] set size to 0
  (`ActorComponent.Deactivate` _boxcollision)
  (`BoxComponent.SetBoxExtent` _boxcollision _reset_size true)
  (`ActorComponent.Deactivate` _cubetexture)
  (`SceneComponent.SetWorldScale3D` _cubetexture _reset_size))

(event `self.BackShieldFire`
  (bind _boxcollision (`self.BoxCollision`))
  (bind _cubetexture (`self.CubeTexture`))
  ;[1 1 1] deployment of shield
  (bind _returnvalue (`self.GetCanShoot`))
  (if _returnvalue
    (`|ExecutionSequence`
      (:`then_0`
        (`self.SetCanShoot` false)
        (`self.SetIsActive` true))
      (:`then_1`
        (`ActorComponent.Activate` _boxcollision true)
        (`ActorComponent.Activate` _cubetexture true))
      (:`then_2`
        (`BoxComponent.SetBoxExtent` _boxcollision (`self.boxCollisionSize`) true)
        (`SceneComponent.SetWorldScale3D` _cubetexture (`self.cubeTextureSize`))))))

(event `KillShield`
  ;[1 1 1] kill Shield (health > 0)
  (`self.Init`)
  (`self.SetIsActive` false)
  (`KismetSystemLibrary.Delay` (`self.maxCooldown`))
  (`self.SetCanShoot` true))

(event `self.BoxCollision.OnComponentBeginOverlap`
  (params (OverlappedComponent :type "PrimitiveComponent Object Reference") (OtherActor :type "Actor Object Reference") (OtherComp :type "PrimitiveComponent Object Reference") (OtherBodyIndex :type Integer) (bFromSweep :type Boolean) (SweepResult :type "HitResult Structure (by ref)"))
  (bind _asbp_homing_missile_cpp (cast `/Game/Design/Weapons/PickupWeapons/Offensive/HomingMissile/BP_HomingMissileCPP` OtherActor)
    (:`then`
      (`self.K2_DestroyActor` _asbp_homing_missile_cpp)
      (`self.ReceiveDamage` (`/Game/Design/Weapons/PickupWeapons/Offensive/HomingMissile/BP_HomingMissileCPP.WeaponDamage` _asbp_homing_missile_cpp)))
    (:`CastFailed`
      (`KismetSystemLibrary.PrintString` "missileCastFailed"))))

(fn `UserConstructionScript`)