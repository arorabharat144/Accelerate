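; Electric fog grenade, a defensive weapon that expands into a damaging, slowing fog sphere around its location.
; After a deploy delay, a timeline grows the collision sphere and visual, and the actor destroys itself once the fog duration elapses.
; Overlapping AcceleratePlayer cars other than the owner are slowed and take damage through a delay loop gated by one shared overlap flag.
; Setters supply owner, damage and duration; the particle effect remains unwired.
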(event `self.ReceiveBeginPlay`
  (`SphereComponent.SetSphereRadius` (`self.Spherecolision`) 0.1 true)
  (`SceneComponent.SetRelativeScale3D` (`self.Spheretext`) (0.1 0.1 0.1))
  (`self.deploy`))

(event `self.ReceiveTick`
  (params (DeltaSeconds :type "Float (single-precision)")))

(event `deploy`
  (`KismetSystemLibrary.Delay` (`self.DelayForExpanding`))
  (bind (_direction _lerpamount) (`Timeline|Timeline_0` :`NewTime` 1.0 :!via `PlayFromStart`)
    (:`Update`
      (`SphereComponent.SetSphereRadius` (`self.Spherecolision`) (`KismetMathLibrary.Lerp` 0.0 (`self.FogSphereSize`) _lerpamount) true)
      (`SceneComponent.SetRelativeScale3D` (`self.Spheretext`) (`KismetMathLibrary.VLerp` (0.1 0.1 0.1) (`self.FogSphereTextureSize`) _lerpamount))
      (`KismetSystemLibrary.Delay` (`self.mFogDuration`))
      (`self.K2_DestroyActor`))))

(event `self.Spherecolision.OnComponentBeginOverlap`
  (params (OverlappedComponent :type "PrimitiveComponent Object Reference") (OtherActor :type "Actor Object Reference") (OtherComp :type "PrimitiveComponent Object Reference") (OtherBodyIndex :type Integer) (bFromSweep :type Boolean) (SweepResult :type "HitResult Structure (by ref)"))
  (`|ExecutionSequence`
    (:`then_0`
      (bind _asaccelerate_player (cast `AcceleratePlayer` OtherActor))
      (if (!= _asaccelerate_player (`self.MyOwner`))
        (`Car.SlowCar` _asaccelerate_player true (`self.SlowAmount`))
        (set `self.isOverlapping` true)
        (`KismetSystemLibrary.Delay` (`self.timeBetweenBamage`) :!label _label)
        (if (`self.isOverlapping`)
          (`self.TimeForDamage` _asaccelerate_player)
          (goto _label))))))

(event `TimeForDamage`
  (params (Car :type "AcceleratePlayer Object Reference"))
  (`AcceleratePlayer.ReceiveDamage` Car (`self.mFogDamage`)))

(event `self.Spherecolision.OnComponentEndOverlap`
  (params (OverlappedComponent :type "PrimitiveComponent Object Reference") (OtherActor :type "Actor Object Reference") (OtherComp :type "PrimitiveComponent Object Reference") (OtherBodyIndex :type Integer))
  (bind _asaccelerate_player (cast `AcceleratePlayer` OtherActor))
  (if (!= _asaccelerate_player (`self.GetOwner`))
    (`Car.SlowCar` _asaccelerate_player false 1.0)
    (set `self.isOverlapping` false)))

(fn `SetDamage&LifeTime`
  (params (FogDuration :type "Float (double-precision)") (FogDamage :type "Float (double-precision)"))
  (set `self.mFogDuration` FogDuration)
  (set `self.mFogDamage` FogDamage))

(fn `setMyAccelerateOwner`
  (params (owner :type "AcceleratePlayer Object Reference"))
  (set `self.MyOwner` owner))

(fn `UserConstructionScript`)