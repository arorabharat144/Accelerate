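; BP_ElectricFog is a defensive weapon that launches electric fog grenades for its owning AcceleratePlayer.
; BeginPlay caches the owner and enables shooting.
; When ElectricFogFire is called and shooting is allowed, it spawns a BP_ElectricFogGrenade at the Barrel transform, passing it the owner and the fog's duration and damage.
; A CanShoot flag and a Delay of MaxCooldown gate repeat shots.
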(event `self.ReceiveBeginPlay`
  (bind _asaccelerate_player (cast `AcceleratePlayer` (`self.GetOwner`)))
  (set `self.OwnerRef` _asaccelerate_player)
  (`self.SetCanShoot` true))

(event `self.ElectricFogFire`
  (bind _returnvalue (`self.GetCanShoot`))
  (if _returnvalue
    (`self.SetCanShoot` false)
    (bind _returnvalue_2 (`|SpawnActorFromClass` "/Game/Design/Weapons/BaseWeapons/Defensive/ElectricFog/BP_ElectricFogGrenade.BP_ElectricFogGrenade_C" (`SceneComponent.K2_GetComponentToWorld` (`self.Barrel`)) "Undefined" "OverrideRootScale" null null))
    (`/Game/Design/Weapons/BaseWeapons/Defensive/ElectricFog/BP_ElectricFogGrenade.setMyAccelerateOwner` _returnvalue_2 (`self.OwnerRef`))
    (`/Game/Design/Weapons/BaseWeapons/Defensive/ElectricFog/BP_ElectricFogGrenade.SetDamage&LifeTime` _returnvalue_2 (`self.mFogDuration`) (`self.mFogDamage`))
    (`KismetSystemLibrary.Delay` (`self.maxCooldown`))
    (`self.SetCanShoot` true)))

(fn `UserConstructionScript`)