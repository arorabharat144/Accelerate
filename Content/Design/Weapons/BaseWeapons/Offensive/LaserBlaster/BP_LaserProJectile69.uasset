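; Laser blaster projectile actor that damages players it overlaps and expires after a short life span.
; On overlap, if the other AcceleratePlayer is not its owning player, it applies Damage and destroys itself.
; AddSpeed sets the movement component's initial speed to BasicSpeed plus the passed speed, while setters take damage and BulletSpeed.
; A dome shield check exists but is disconnected.
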(event `self.ReceiveBeginPlay`
  ;[1 1 1] Set Laser Life Span
  (`self.SetLifeSpan` 5.0))

(event `self.ReceiveActorBeginOverlap`
  (params (OtherActor :type "Actor Object Reference"))
  ;[1 1 1] Deal Damage to BP_Car
  (bind _asaccelerate_player (cast `AcceleratePlayer` OtherActor))
  (bind _asaccelerate_player_2 (cast `AcceleratePlayer` (`self.GetOwner` self)))
  (if (!= _asaccelerate_player_2 _asaccelerate_player)
    (`AcceleratePlayer.ReceiveDamage` _asaccelerate_player (`self.Damage`))
    (`self.K2_DestroyActor`)))

(event `AddSpeed`
  (params (speed :type "Float (double-precision)"))
  ;[1 1 1] Modify Inital speed with Basic Speed
  (set `ProjectileMovementComponent.InitialSpeed` (+ (`self.BasicSpeed`) speed) (`self.ProjectileMovement`)))

(fn `SetLaserDamage`
  (params (damage :type "Float (double-precision)"))
  (set `self.Damage` damage))

(fn `SetLaserSpeed`
  (params (Speed :type "Float (double-precision)"))
  (set `self.BulletSpeed` Speed))

(fn `UserConstructionScript`)