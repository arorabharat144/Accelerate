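; BP_RailGun is an offensive weapon that fires BP_Armature projectiles from its barrel.
; Each tick it derives its own speed from the change in actor location.
; On the fire event, unless heat exceeds the maximum, it spawns the armature at EndOfBarrel, plays the laser sound and passes that speed and the weapon damage to the projectile.
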(event `self.ReceiveBeginPlay`
  ;[1 1 1] Set Position
  (set `self.oldPosition` (`self.K2_GetActorLocation`)))

(event `self.ReceiveTick`
  (params (DeltaSeconds :type "Float (single-precision)"))
  ;[1 1 1] Get car speed and set laser speed
  (set `self.Speed` (/ (`KismetMathLibrary.VSize` (- (`self.K2_GetActorLocation`) (`self.oldPosition`))) (`GameplayStatics.GetWorldDeltaSeconds`)))
  (set `self.oldPosition` (`self.K2_GetActorLocation`)))

(event `self.RailGunBlasterFireEvent`
  ;[1 1 1] Spawn Laser when fired, play sound and set damage
  (if (not (> (`self.mCurrentHeatLevel`) (`self.mMaxHeatLevel`)))
    (`PrimitiveComponent.GetPhysicsLinearVelocity` (`self.GunMesh`) "None")
    (bind _returnvalue (`|SpawnActorFromClass` "/Game/Design/Weapons/BaseWeapons/Offensive/RailGun/BP_Armature.BP_Armature_C" (`SceneComponent.K2_GetComponentToWorld` (`self.EndOfBarrel`)) "Undefined" "OverrideRootScale" null null))
    (`GameplayStatics.PlaySoundAtLocation` (`self.LaserSound`) (`SceneComponent.K2_GetComponentLocation` (`/Game/Design/Weapons/BaseWeapons/Offensive/RailGun/BP_Armature.ArmatureMesh` _returnvalue)) (struct) 1.0 1.0 0.0 null null null)
    (`/Game/Design/Weapons/BaseWeapons/Offensive/RailGun/BP_Armature.SetArmatureSpeed` _returnvalue (`self.Speed`))
    (`/Game/Design/Weapons/BaseWeapons/Offensive/RailGun/BP_Armature.SetArmatureDamage` _returnvalue (`self.mDamage`))))

(fn `UserConstructionScript`)