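; Railgun projectile that damages any AcceleratePlayer it overlaps and then destroys itself.
; On BeginPlay it enables overlap events on its collision and mesh and sets a short life span.
; Other overlapped actors are ignored, as the player cast fails.
; Setters supply damage and base speed, and AddSpeed sets the projectile movement's InitialSpeed to that base plus a passed-in speed.
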(event `self.ReceiveBeginPlay`
  ;[1 1 1] Set Laser Life Span
  (`self.SetLifeSpan` 5.0)
  (set `PrimitiveComponent.bGenerateOverlapEvents` true (`self.ProjectileCollision`))
  (set `PrimitiveComponent.bGenerateOverlapEvents` true (`self.ArmatureMesh`)))

(event `self.ReceiveActorBeginOverlap`
  (params (OtherActor :type "Actor Object Reference"))
  ;[1 1 1] Deal Damage to BP_Car
  (if (not (== OtherActor self))
    (bind _asaccelerate_player (cast `AcceleratePlayer` OtherActor))
    (`AcceleratePlayer.ReceiveDamage` _asaccelerate_player (`self.Damage`))
    (`self.K2_DestroyActor`)))

(event `AddSpeed`
  (params (speed :type "Float (double-precision)"))
  ;[1 1 1] Modify Inital speed with Basic Speed
  (set `ProjectileMovementComponent.InitialSpeed` (+ (`self.BasicSpeed`) speed) (`self.ProjectileMovement`)))

(fn `SetArmatureDamage`
  (params (Damage :type "Float (double-precision)"))
  (set `self.Damage` Damage))

(fn `SetArmatureSpeed`
  (params (Speed :type "Float (double-precision)"))
  (set `self.BasicSpeed` Speed))

(fn `UserConstructionScript`)