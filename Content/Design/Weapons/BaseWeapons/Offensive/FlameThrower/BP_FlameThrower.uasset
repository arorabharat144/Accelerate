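; BP_FlameThrower is an offensive weapon Blueprint whose graph handles flamethrower audio.
; A looping half-second timer from BeginPlay checks whether the flamethrower is active, then branches on an in-use flag.
; If not in use, it plays the ignition sound at the mesh and starts a timeline driving the burning sound's volume.
; If already in use, it reverses that timeline from the end; the timeline clears the flag on finishing.
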(event `self.ReceiveBeginPlay`
  ;[1 1 1] Repeat constant flamethrower
  (`KismetSystemLibrary.K2_SetTimerDelegate` (delegate `Play Flamethrower Sound`) 0.5 true))

(event `Play Flamethrower Sound`
  ;[1 1 1] Repeat constant flamethrower
  (if (`ActorComponent.IsActive` (`self.mFlameThrower`))
    (if (`self.IsUsingFlamethrower`)
      (bind (_direction _flamethrower_volume) (`Timeline|TL_Flamethrower` :!via `ReverseFromEnd` :!label _label)
        (:`Update`
          (set `AudioComponent.VolumeMultiplier` _flamethrower_volume (`self.Burning`)))
        (:`Finished`
          (set `self.IsUsingFlamethrower` false)))
      (else
        (`GameplayStatics.PlaySoundAtLocation` (`self.InitialFlamethrowerSound`) (`SceneComponent.K2_GetComponentLocation` (`self.mFlameThrowerMesh`)) (struct) 1.0 1.0 0.0 null null null)
        (set `self.IsUsingFlamethrower` true)
        (goto _label :!via `PlayFromStart`)))))

(fn `UserConstructionScript`)