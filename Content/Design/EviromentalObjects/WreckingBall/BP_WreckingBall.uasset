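; BP_WreckingBall is a wrecking ball environmental object configured through rope length, ball size, starting rotation and mass.
; The construction script stretches the rope base by length and rolls it to the set angle.
; It scales the ball, offsets it downward by rope length times ball size, and applies one mass scale to rope and ball.
; The event graph has no runtime logic.
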(event `self.ReceiveBeginPlay`)

(fn `UserConstructionScript`
  (bind _ballsize (`self.BallSize`))
  (`SceneComponent.SetWorldScale3D` (`self.RopeBase`) (`KismetMathLibrary.MakeVector` 1.0 1.0 (* (`self.RopeLength`) 0.1)))
  (`SceneComponent.K2_SetRelativeRotation` (`self.RopeBase`) (`KismetMathLibrary.MakeRotator` (`self.BallRotation`)) false false)
  (`SceneComponent.SetWorldScale3D` (`self.WreckingBall`) (`KismetMathLibrary.MakeVector` _ballsize _ballsize _ballsize))
  (`SceneComponent.K2_SetRelativeLocation` (`self.WreckingBall`) (`KismetMathLibrary.MakeVector` 0.0 0.0 (* (`self.RopeLength`) (`self.BallSize`) -2.5)) false false)
  (`PrimitiveComponent.SetMassScale` (`self.Rope`) "None" (`self.BallMass`))
  (`PrimitiveComponent.SetMassScale` (`self.WreckingBall`) "None" (`self.BallMass`)))