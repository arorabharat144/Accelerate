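; BP_ExplodingBarrel is an environmental barrel that explodes when a car or homing missile touches it.
; Its Collision component's begin-overlap event checks whether the other actor's class derives from BP_Car or BP_HomingMissileCPP.
; On a match it spawns a scaled explosion particle at the barrel, fires the Explosion component's impulse, plays a sound and destroys itself.
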(event `self.Collision.OnComponentBeginOverlap`
  (params (OverlappedComponent :type "PrimitiveComponent Object Reference") (OtherActor :type "Actor Object Reference") (OtherComp :type "PrimitiveComponent Object Reference") (OtherBodyIndex :type Integer) (bFromSweep :type Boolean) (SweepResult :type "HitResult Structure (by ref)"))
  (bind _returnvalue (`GameplayStatics.GetObjectClass` OtherActor))
  (bind _explosionsize (`self.ExplosionSize`))
  ;[1 1 1] Check if actor is BP_Car
  (if (or (`KismetMathLibrary.ClassIsChildOf` _returnvalue "/Game/Design/Car/BP_Car.BP_Car_C") (`KismetMathLibrary.ClassIsChildOf` _returnvalue "/Game/Design/Weapons/PickupWeapons/Offensive/HomingMissile/BP_HomingMissileCPP.BP_HomingMissileCPP_C"))
    (`GameplayStatics.SpawnEmitterAtLocation` (`self.ExplosionParticle`) (`SceneComponent.K2_GetComponentLocation` (`self.Barrel`)) (struct) (`KismetMathLibrary.MakeVector` _explosionsize _explosionsize _explosionsize))
    (`RadialForceComponent.FireImpulse` (`self.Explosion`))
    (`GameplayStatics.PlaySoundAtLocation` (`self.ExplosionSound`) (`SceneComponent.K2_GetComponentLocation` (`self.Barrel`)) (struct) 1.0 1.0 0.0 null null null)
    (`self.K2_DestroyActor`)))

(fn `UserConstructionScript`)