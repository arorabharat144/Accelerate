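; Sawblade environmental object that spins its blade while shuttling between its Base and a MoveLocation marker.
; From BeginPlay, the SawMovement and Timeline_0 timelines restart each other in an endless loop, each lerping BladeBase's world location without sweep.
; Tick pitches the Sawblade locally by DeltaSeconds plus RotateSpeed, added rather than multiplied, so spin speed depends on frame rate.
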(event `self.ReceiveBeginPlay`
  (bind (_direction _alpha) (`Timeline|SawMovement` :!via `PlayFromStart` :!label _label)
    (:`Update`
      (`SceneComponent.K2_SetWorldLocation` (`self.BladeBase`) (`KismetMathLibrary.VLerp` (`SceneComponent.K2_GetComponentLocation` (`self.Base`)) (`SceneComponent.K2_GetComponentLocation` (`self.MoveLocation`)) _alpha) false false))
    (:`Finished`
      (bind (_direction_2 _alpha_2) (`Timeline|Timeline_0` :!via `PlayFromStart`)
        (:`Update`
          (`SceneComponent.K2_SetWorldLocation` (`self.BladeBase`) (`KismetMathLibrary.VLerp` (`SceneComponent.K2_GetComponentLocation` (`self.Base`)) (`SceneComponent.K2_GetComponentLocation` (`self.MoveLocation`)) _alpha_2) false false))
        (:`Finished`
          (goto _label :!via `PlayFromStart`))))))

(event `self.ReceiveTick`
  (params (DeltaSeconds :type "Float (single-precision)"))
  (`SceneComponent.K2_AddLocalRotation` (`self.Sawblade`) (`KismetMathLibrary.MakeRotator` 0.0 (+ DeltaSeconds (`self.RotateSpeed`))) false false))

(fn `UserConstructionScript`)