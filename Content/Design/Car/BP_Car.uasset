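; BP_Car is the car Blueprint, handling boost effects, engine audio and a translucent phase look.
; Boost input sets boost flags and activates the tire effects, which shut off on release or when boost runs out.
; Tick feeds speed into the engine audio's RPM parameter.
; A C++-called event swaps each material for a translucent dynamic instance, copying its textures and lowering alpha, then restores the originals when phasing ends.
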(event `InputAction|BoostParticle`
  (params (Key :type "Key Structure"))
  (bind _righttire (`self.RightTire`))
  ;[0.09412 0.7373 1] Activate Boost
  (:`Pressed`
    (bind _output_get (set `self.IsBoosted` true))
    (if (and _output_get (> (`self.mBoostCurrent`) 0.0))
      (`ActorComponent.Activate` _righttire true)
      (`ActorComponent.Activate` (`self.LeftTire`) true)
      (set `self.CanBoost` true)))
  (:`Released`
    (set `self.IsBoosted` false)
    (`ActorComponent.Deactivate` _righttire)
    (`ActorComponent.Deactivate` (`self.LeftTire`))
    (set `self.CanBoost` false)))

(event `self.ReceiveTick`
  (params (DeltaSeconds :type "Float (single-precision)"))
  ;[0.4235 0.3765 0.4471] Update / Event Tick
  (`|ExecutionSequence`
    (:`then_2`
      ;[1 0.2627 0] Audio
      (`AudioComponent.SetFloatParameter` (`self.EngineAudio`) "RPM" (`KismetMathLibrary.Abs` (* (`KismetMathLibrary.VSize` (`self.GetVelocity`)) 0.036))))
    (:`then_3`
      (if (<= (`self.mBoostCurrent`) 0.0)
        (`ActorComponent.Deactivate` (`self.LeftTire`))
        (`ActorComponent.Deactivate` (`self.RightTire`))
        (set `self.CanBoost` false)))))

(event `ApplyPhaseMaterial`
  (params (active :type Boolean))
  ;[1 1 1] Phase Material Effect - Event called by C++
  (if active
    ;;[1 1 1] Temp array of car materials
    (bind _output_get (set `self.OrigCarMaterials` (`MeshComponent.GetMaterials` (`self.Mesh`))))
    (for (_array_element _array_index) _output_get
      ;;[1 1 1] Create Dynamic Transparent Material
      (bind _returnvalue (`PrimitiveComponent.CreateDynamicMaterialInstance` (`self.Mesh`) _array_index "/Game/Design/Car/Materials/TranslucentMaterial.TranslucentMaterial" "None"))
      (`|ExecutionSequence`
        (:`then_0`
          ;;[1 1 1] Loop through texture params
          (for _array_element_2 (`self.TextureParameters`)
            (bind _asmaterial_instance_constant (cast `MaterialInstanceConstant` _array_element))
            (bind _returnvalue_2 (`MaterialInstanceConstant.K2_GetTextureParameterValue` _asmaterial_instance_constant _array_element_2))
            (`MaterialInstanceDynamic.SetTextureParameterValue` _returnvalue _array_element_2 _returnvalue_2)))
        (:`then_1`
          ;;[1 1 1] Set the Alpha amount on the dynamic material
          (`MaterialInstanceDynamic.SetScalarParameterValue` _returnvalue "AlphaMod" 0.2))))
    (else
      (for (_array_element_3 _array_index_2) (`self.OrigCarMaterials`)
        (`PrimitiveComponent.SetMaterial` (`self.Mesh`) _array_index_2 _array_element_3)))))

(fn `UserConstructionScript`)